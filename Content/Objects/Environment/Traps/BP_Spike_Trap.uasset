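; BP_Spike_Trap is a configurable environment trap that becomes spikes, hatch, spinning fire dragon or gas, despite its name.
; Construction and delayed BeginPlay use TrapId, or a random pick when -1, to swap the floor mesh and build instanced body and element meshes.
; Collider overlap or cursor hover plays the matching animation behind an InUse guard.
; Animations chain component moves, task delays and effect toggles; no damage is applied here.
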(event `self.ReceiveBeginPlay`
  (`InstancedStaticMeshComponent.ClearInstances` (`self.Trap_Body`))
  (`InstancedStaticMeshComponent.ClearInstances` (`self.Trap_Hatch_Door1`))
  (`InstancedStaticMeshComponent.ClearInstances` (`self.Trap_Spikes`))
  (`InstancedStaticMeshComponent.ClearInstances` (`self.Trap_Hatch_Door2`))
  (`InstancedStaticMeshComponent.ClearInstances` (`self.Trap_Dragon`))
  (bind _returnvalue (`AddComponent|NODE_AddGameplayTasksComponent-3`))
  (`GameplayTask_WaitDelay.TaskWaitDelay` _returnvalue 0.1
    (:`then`
      (`self.Set_Trap_ID`)
      (`self.Spawn_mesh_instance`))))

(event `self.ReceiveActorBeginOverlap`
  (params (OtherActor :type "Actor Object Reference")))

(event `self.Collider.OnComponentBeginOverlap`
  (params (OverlappedComponent :type "PrimitiveComponent Object Reference") (OtherActor :type "Actor Object Reference") (OtherComp :type "PrimitiveComponent Object Reference") (OtherBodyIndex :type Integer) (bFromSweep :type Boolean) (SweepResult :type "HitResult Structure (by ref)"))
  (if (not (`self.InUse`)) :!label _label
    (set `self.InUse` true)
    (switch `int` (`|GetArrayItem` (`self.Trap_Animation_ID`) (`self.Trap_id_now`))
      (:`0`
        (`self.Spike_Anim`
          (:`NewParam`
            _)))
      (:`1`
        (`self.Hatch_Anim`
          (:`NewParam`
            _)))
      (:`2`
        (`self.Dragon_Anim`))
      (:`4`
        (`self.Gass_Anim`)))
    (set `self.InUse` false)))

(event `self.Collider.OnBeginCursorOver`
  (params (TouchedComponent :type "PrimitiveComponent Object Reference"))
  (goto _label))

(fn `Set_Trap_ID`
  (returns (Trap_id_now :type Integer))
  (bind _trap_id (`self.Trap_id`))
  (bind _returnvalue (`KismetArrayLibrary.Array_Length` (`self.Trap_Body_Array`)))
  (bind _output_get (set `self.Rand_Stream` (`KismetMathLibrary.MakeRandomStream` (`KismetMathLibrary.RandomInteger` 2147483647))))
  (if (== _returnvalue 0)
    _
    (elif (== _trap_id -1.0)
      (bind _output_get_2 (set `self.Trap_id_now` (`KismetMathLibrary.RandomIntegerInRangeFromStream` _output_get 0 (- _returnvalue 1))))
      (return _output_get_2)
      (else
        (bind _output_get_3 (set `self.Trap_id_now` _trap_id))
        (return _output_get_3)))))

(fn `Spawn_mesh_instance`
  (locals (Hatch :type String :default "hatch_") (Spike :type String :default "spike_") (Meshes :type "/Game/Objects/Environment/Floor/Floor_Trap_Holes_Meshes Structure") (Dragon :type String :default "dragon_") (Gass :type String :default "Gass_"))
  (bind _default_position (`self.Default_position`))
  (bind _trap_body (`self.Trap_Body`))
  (bind _trap_hatch_door1 (`self.Trap_Hatch_Door1`))
  (bind _trap_hatch_door2 (`self.Trap_Hatch_Door2`))
  (bind _trap_dragon (`self.Trap_Dragon`))
  (bind _trap_id_now (`self.Trap_id_now`))
  (bind _default_position_2 (`self.Default_position`))
  (bind _traptagwhile (`self.TrapTagWhile`))
  (bind _trap_id_now_2 (`self.Trap_id_now`))
  (bind _meshes_trap_holes_types (break `/Game/Objects/Environment/Floor/Floor_Trap_Holes_Meshes` (`local.Meshes`)))
  (bind _trap_id_now_3 (`self.Trap_id_now`))
  (bind _default_position_3 (`self.Default_position`))
  (bind _trap_body_2 (`self.Trap_Body`))
  (bind _trap_body_3 (`self.Trap_Body`))
  (bind _trap_body_4 (`self.Trap_Body`))
  (bind _trap_spikes (`self.Trap_Spikes`))
  (bind (_min _max) (`StaticMeshComponent.GetLocalBounds` _trap_spikes))
  (bind _value (`self.Get_Randomiset_Ellement` (`local.Hatch`) (`|GetArrayItem` (`self.Trap_Ellement_id`) _trap_id_now)))
  ;[1 1 1] Get Floor ID
  (bind _asstatic_mesh_component (cast `StaticMeshComponent` (`|GetArrayItem` (`SceneComponent.GetChildrenComponents` (`|GetArrayItem` (`SceneComponent.GetChildrenComponents` (`self.BP_Floor`) false)) false) _traptagwhile) :!label _label)
    (:`then`
      (set `self.TrapTagWhile` 0)
      ;[1 1 1] Set new floor
      (`StaticMeshComponent.SetStaticMesh` _asstatic_mesh_component (`|GetArrayItem` _meshes_trap_holes_types (`|GetArrayItem` (`self.Floor_By_ID`) (`self.Trap_id_now`))))
      (switch `int` (`|GetArrayItem` (`self.Trap_Animation_ID`) (`self.Trap_id_now`))
        (:`0`
          ;[1 1 1] Spikess
          (`StaticMeshComponent.SetStaticMesh` _trap_body_3 (`|GetArrayItem` (`self.Trap_Body_Array`) _trap_id_now_3))
          (`InstancedStaticMeshComponent.AddInstance` _trap_body_3 _default_position_2 false)
          (`StaticMeshComponent.SetStaticMesh` _trap_spikes (`self.Get_Randomiset_Ellement` (`local.Spike`) (`|GetArrayItem` (`self.Trap_Ellement_id`) _trap_id_now_3)))
          (`InstancedStaticMeshComponent.AddInstance` _trap_spikes (`KismetMathLibrary.MakeTransform` (`KismetMathLibrary.MakeVector` (.x (.location _default_position_2)) (.y (.location _default_position_2)) (- (.z (.location _default_position_2)) (+ (- (.z _max) (.z _min)) (`|GetArrayItem` (`self.Trap_Ellement_Offset`) _trap_id_now_3))))) false))
        (:`1`
          ;[1 1 1] Hatch
          (`StaticMeshComponent.SetStaticMesh` _trap_body_4 (`|GetArrayItem` (`self.Trap_Body_Array`) _trap_id_now))
          (`InstancedStaticMeshComponent.AddInstance` _trap_body_4 _default_position false)
          (`StaticMeshComponent.SetStaticMesh` _trap_hatch_door1 _value)
          (`StaticMeshComponent.SetStaticMesh` _trap_hatch_door2 _value)
          (`InstancedStaticMeshComponent.AddInstance` _trap_hatch_door1 _default_position false)
          (`InstancedStaticMeshComponent.AddInstance` _trap_hatch_door2 _default_position false))
        (:`2`
          ;[1 1 1] Dragon
          (`StaticMeshComponent.SetStaticMesh` _trap_body_2 (`|GetArrayItem` (`self.Trap_Body_Array`) _trap_id_now_2))
          (`InstancedStaticMeshComponent.AddInstance` _trap_body_2 _default_position_3 false)
          (`StaticMeshComponent.SetStaticMesh` _trap_dragon (`self.Get_Randomiset_Ellement` (`local.Dragon`) (`|GetArrayItem` (`self.Trap_Ellement_id`) _trap_id_now_2)))
          (`InstancedStaticMeshComponent.AddInstance` _trap_dragon _default_position_3 false))
        (:`4`
          ;[1 1 1] Dragon
          (`StaticMeshComponent.SetStaticMesh` _trap_body (`|GetArrayItem` (`self.Trap_Body_Array`) (`self.Trap_id_now`)))
          (`InstancedStaticMeshComponent.AddInstance` _trap_body (`self.Default_position`) false)))
      (return))
    (:`CastFailed`
      (set `self.TrapTagWhile` (+ _traptagwhile 1))
      (goto _label))))

(fn `UserConstructionScript`
  (locals (Reaction_Name :type "Array of String"))
  (`self.Set_Trap_ID`)
  (`self.Spawn_mesh_instance`))